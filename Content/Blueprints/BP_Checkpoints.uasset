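; Checkpoint actor that tracks progress around a timed lap through four ordered overlap zones.
; Checkpoint1 serves as start and finish, adding the timer HUD widget at count zero and setting StopTimer at count four.
; Checkpoints 2–4 pass the TrackCheckpoint counter through CheckCheckpoint, which returns it incremented only on a match, with no explicit value otherwise.
; Overlaps print the counter, except at the finish.
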(event `self.Checkpoint1.OnComponentBeginOverlap`
  (params (OverlappedComponent :type "PrimitiveComponent Object Reference") (OtherActor :type "Actor Object Reference") (OtherComp :type "PrimitiveComponent Object Reference") (OtherBodyIndex :type Integer) (bFromSweep :type Boolean) (SweepResult :type "HitResult Structure (by ref)"))
  ; Checks if the right checkpoint has been crossed;
  (switch `int` (`self.trackCheckpoint`)
    (:`0`
      (bind _result (`/Engine/EditorBlueprintResources/StandardMacros.IncrementInt` (`self.trackCheckpoint`))
        (:`  `
          (bind _output_get (set `self.trackCheckpoint` _result))
          (`KismetSystemLibrary.PrintText` (`KismetTextLibrary.Conv_IntToText` _output_get))
          ; Adds timer to HUD
          (bind _returnvalue (`|CreateWidget` "/Game/Blueprints/WBP_TimerHUD.WBP_TimerHUD_C"))
          (`UserWidget.AddToViewport` _returnvalue 0))))
    (:`4`
      ; Stops timer
      (set `self.StopTimer` true)
      (bind _result_2 (`/Engine/EditorBlueprintResources/StandardMacros.IncrementInt` (`self.trackCheckpoint`))
        (:`  `
          (set `self.trackCheckpoint` _result_2))))))

(event `self.Checkpoint2.OnComponentBeginOverlap`
  (params (OverlappedComponent :type "PrimitiveComponent Object Reference") (OtherActor :type "Actor Object Reference") (OtherComp :type "PrimitiveComponent Object Reference") (OtherBodyIndex :type Integer) (bFromSweep :type Boolean) (SweepResult :type "HitResult Structure (by ref)"))
  ; Checks if the right checkpoint has been crossed
  (bind _return (`self.CheckCheckpoint` (`self.trackCheckpoint`) 1))
  (bind _output_get (set `self.trackCheckpoint` _return))
  (`KismetSystemLibrary.PrintText` (`KismetTextLibrary.Conv_IntToText` _output_get)))

(event `self.Checkpoint3.OnComponentBeginOverlap`
  (params (OverlappedComponent :type "PrimitiveComponent Object Reference") (OtherActor :type "Actor Object Reference") (OtherComp :type "PrimitiveComponent Object Reference") (OtherBodyIndex :type Integer) (bFromSweep :type Boolean) (SweepResult :type "HitResult Structure (by ref)"))
  ; Checks if the right checkpoint has been crossed
  (bind _return (`self.CheckCheckpoint` (`self.trackCheckpoint`) 2))
  (bind _output_get (set `self.trackCheckpoint` _return))
  (`KismetSystemLibrary.PrintText` (`KismetTextLibrary.Conv_IntToText` _output_get)))

(event `self.Checkpoint4.OnComponentBeginOverlap`
  (params (OverlappedComponent :type "PrimitiveComponent Object Reference") (OtherActor :type "Actor Object Reference") (OtherComp :type "PrimitiveComponent Object Reference") (OtherBodyIndex :type Integer) (bFromSweep :type Boolean) (SweepResult :type "HitResult Structure (by ref)"))
  ; Checks if the right checkpoint has been crossed
  (bind _return (`self.CheckCheckpoint` (`self.trackCheckpoint`) 3))
  (bind _output_get (set `self.trackCheckpoint` _return))
  (`KismetSystemLibrary.PrintText` (`KismetTextLibrary.Conv_IntToText` _output_get)))

(fn `CheckCheckpoint`
  (params (Zone :type Integer) (Checkpoint :type Integer))
  (returns (return :type Integer))
  ; Checks if Zone == Checkpoint, if true zone incremented and returned else nothing
  (if (== Zone Checkpoint)
    (bind _result (`/Engine/EditorBlueprintResources/StandardMacros.IncrementInt` Zone)
      (:`  `
        (return _result)))))

(fn `UserConstructionScript`)